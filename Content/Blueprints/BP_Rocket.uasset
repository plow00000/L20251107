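; BP_Rocket is a projectile actor that flies forward along its local X axis at Speed and expires after a set lifespan.
; On overlapping any actor, it applies damage to it, then spawns a scaled explosion emitter and sound at its position.
; It then asks BP_GameMode to check the remaining target count and destroys itself, though the destroy only runs if the game mode cast succeeds.
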(event `self.ReceiveBeginPlay`
  ; 삭제 시간 설정
  (`self.SetLifeSpan` 10.0))

(event `self.ReceiveTick`
  (params (DeltaSeconds :type "Float (single-precision)"))
  ; 전진
  (`self.K2_AddActorLocalOffset` (`KismetMathLibrary.MakeVector` (* DeltaSeconds (`self.Speed`)))))

(event `self.ReceiveActorBeginOverlap`
  (params (OtherActor :type "Actor Object Reference"))
  (bind (_returnvalue_location _returnvalue_rotation _returnvalue_scale) (`KismetMathLibrary.BreakTransform` (`self.GetTransform`)))
  (`|ExecutionSequence`
    (:`then_0`
      (`GameplayStatics.ApplyDamage` OtherActor 100.0 (`self.GetInstigatorController`) self))
    (:`then_1`
      (`GameplayStatics.SpawnEmitterAtLocation` "/Game/StarterContent/Particles/P_Explosion.P_Explosion" _returnvalue_location _returnvalue_rotation (* _returnvalue_scale 1.5))
      (`GameplayStatics.SpawnSoundAtLocation` "/Game/StarterContent/Audio/Explosion_Cue_01.Explosion_Cue_01" (`self.K2_GetActorLocation`) (struct) 1.0 1.0 0.0 null null)
      ; 남은 타겟 수 확인해달라고 요청
      (bind _asbp_game_mode (cast `/Game/GameModes/BP_GameMode` (`GameplayStatics.GetGameMode`)))
      (`/Game/GameModes/BP_GameMode.CheckTargetAmount` _asbp_game_mode)
      (`self.K2_DestroyActor`))))

(fn `UserConstructionScript`)