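; BP_P38 is a player-controlled P-38 plane pawn that flies forward continuously and fires rockets.
; Tick feeds movement input along the Arrow component's forward vector, scaled by Speed.
; Enhanced Input IA_Move applies local roll from X and pitch from Y, scaled by delta time, with no yaw control.
; IA_Fire spawns BP_Rocket at the Arrow's world transform, with the plane as owner and instigator.
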(event `self.ReceiveTick`
  (params (DeltaSeconds :type "Float (single-precision)"))
  ; 이동
  (`self.AddMovementInput` (`SceneComponent.GetForwardVector` (`self.Arrow`)) (`self.Speed`)))

(event `EnhancedInput|/Game/Input/IA_Fire`
  (params (ActionValue :type Boolean) (ElapsedSeconds :type "Float (double-precision)") (TriggeredSeconds :type "Float (double-precision)") (InputAction :type "InputAction Object Reference" :default "/Game/Input/IA_Fire.IA_Fire"))
  ; 공격
  (:`Triggered`
    (`|SpawnActorFromClass` "/Game/Blueprints/BP_Rocket.BP_Rocket_C" (`SceneComponent.K2_GetComponentToWorld` (`self.Arrow`)) "AlwaysSpawn" "MultiplyWithRoot" self self)))

(event `EnhancedInput|/Game/Input/IA_Move`
  (params (ActionValue :type "Vector2D Structure") (ElapsedSeconds :type "Float (double-precision)") (TriggeredSeconds :type "Float (double-precision)") (InputAction :type "InputAction Object Reference" :default "/Game/Input/IA_Move.IA_Move"))
  ; 방향 전환
  (:`Triggered`
    (`|ExecutionSequence`
      (:`then_0`
        (`self.K2_AddActorLocalRotation` (`KismetMathLibrary.MakeRotator` (* ActionValue_X 30.0 (`GameplayStatics.GetWorldDeltaSeconds`)))))
      (:`then_1`
        (`self.K2_AddActorLocalRotation` (`KismetMathLibrary.MakeRotator` 0.0 (* ActionValue_Y 30.0 (`GameplayStatics.GetWorldDeltaSeconds`))))))))

(fn `UserConstructionScript`)