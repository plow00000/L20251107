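; BP_GameMode is the game mode that handles level progression once all targets are gone.
; Its CheckTargetAmount event counts BP_Target actors and, when none remain, waits briefly before checking the current level name.
; A switch on that name opens the next hard-coded level for levels 01 through 03, while Lvl_Main reloads itself and Level 04 has no case.
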(event `CheckTargetAmount`
  (bind _outactors (`GameplayStatics.GetAllActorsOfClass` "/Game/Blueprints/BP_Target.BP_Target_C"))
  (if (not (`KismetMathLibrary.Conv_IntToBool` (`KismetArrayLibrary.Array_Length` _outactors)))
    (`KismetSystemLibrary.Delay` 1.0)
    (bind _returnvalue (`GameplayStatics.GetCurrentLevelName` true))
    (switch `string` _returnvalue
      (:`Lvl_Main`
        (`GameplayStatics.OpenLevel` "Lvl_Main"))
      (:`Lvl_Level_01`
        (`GameplayStatics.OpenLevel` "Lvl_Level_02"))
      (:`Lvl_Level_02`
        (`GameplayStatics.OpenLevel` "Lvl_Level_03"))
      (:`Lvl_Level_03`
        (`GameplayStatics.OpenLevel` "Lvl_Level_04")))))

(fn `UserConstructionScript`)